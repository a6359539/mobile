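; BP_wateraiController is an AI controller that starts the BP_waterair behavior tree, apparently for a water animal.
; BeginPlay and OnPossess both run the same setup, which loads BP_AnimalBB and seeds its home location and idle time keys.
; A random navigable point near the controller's own location, rather than the pawn's, becomes the initial target before the tree runs.
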(event `self.ReceiveBeginPlay`
  (bind _returnvalue (`self.K2_GetActorLocation`))
  (bind (_randomlocation _returnvalue_2) (`NavigationSystem.K2_GetRandomLocationInNavigableRadius` _returnvalue 500.0))
  (`|ExecutionSequence` :!label _label
    (:`then_0`
      (`self.UseBlackboard` "/Game/wonseok/AIController/BP_AnimalBB.BP_AnimalBB")
      (`BlackboardComponent.SetValueAsVector` (`self.Blackboard`) (`self.HomeLocKey`) _returnvalue)
      (`BlackboardComponent.SetValueAsFloat` (`self.Blackboard`) (`self.IdleTimeKey`) 4.0)
      (if _returnvalue_2
        (`BlackboardComponent.SetValueAsVector` (`self.Blackboard`) (`self.TargetLocKey`) _randomlocation)))
    (:`then_1`
      (`self.RunBehaviorTree` "/Game/wonseok/AIController/BP_waterair.BP_waterair"))))

(event `self.OnPossess`
  (params (PossessedPawn :type "Pawn Object Reference"))
  (goto _label))

(fn `UserConstructionScript`)